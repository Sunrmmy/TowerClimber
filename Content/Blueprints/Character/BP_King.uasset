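; BP_King is the King character Blueprint, set up for Enhanced Input with a platformer mapping context.
; On BeginPlay, it casts its controller to PlayerController and adds IMC_Platformer to that player's Enhanced Input subsystem.
; The Jump and Move input actions only print debug strings when started, with no movement or jump logic in this graph.
; The construction script only calls its parent.
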(event Input|EnhancedActionEvents|EnhancedInputActionIA_Jump
  (params (ActionValue :type Boolean) (ElapsedSeconds :type Float%20%28double-precision%29) (TriggeredSeconds :type Float%20%28double-precision%29) (InputAction :type Input%20Action%20Object%20Reference :default "/Game/Input/Actions/IA_Jump.IA_Jump"))
  (:Started
    (Development|PrintString "Jump")))

(event Input|EnhancedActionEvents|EnhancedInputActionIA_Move
  (params (ActionValue :type Float%20%28double-precision%29) (ElapsedSeconds :type Float%20%28double-precision%29) (TriggeredSeconds :type Float%20%28double-precision%29) (InputAction :type Input%20Action%20Object%20Reference :default "/Game/Input/Actions/IA_Move.IA_Move"))
  (:Started
    (Development|PrintString "Move")))

(event EventBeginPlay
  (|CallParentFunction)
  (bind _as玩家控制器 (Utilities|Casting|CastToPlayerController (Pawn|GetController)))
  (Input|AddMappingContext (PlayerController|LocalPlayerSubsystems|GetEnhancedInputLocalPlayerSubsystem _as玩家控制器) "/Game/Input/IMC_Platformer.IMC_Platformer" 0 "(bIgnoreAllPressedKeysUntilRelease=True,bForceImmediately=False,bNotifyUserSettings=False)"))

(fn ConstructionScript
  (|CallParentFunction))